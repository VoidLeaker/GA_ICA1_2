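; BP_BlueDoor is a sliding door that opens while enough pressure switches are active.
; SwitchActivate and SwitchDeactive adjust the active count, then play or reverse the DoorOpen timeline against the required number.
; The timeline lerps the mesh's X from its current world position toward a hardcoded target, applied as relative location with fixed Y and Z.
; A box overlap by BP_ThirdPersonCharacter plays a denied sound, regardless of door state.
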(event `SwitchActivate`
  (bind _staticmeshcomponent (`self.StaticMeshComponent`))
  (bind _returnvalue_x (`KismetMathLibrary.BreakVector` (`SceneComponent.K2_GetComponentLocation` _staticmeshcomponent)))
  ;[0 1 0.9212 0.5 40] Door gets activate once the pressure plate is stepped on (Different version of OrangeDoor opening)
  (`/Engine/EditorBlueprintResources/StandardMacros.IncrementInt` (`self.PressureSwitchActive`)
    (:`  `
      (if (>= (`self.PressureSwitchActive`) (`self.PressureSwitchNeeded`))
        (bind (_direction _sliding) (`Timeline|DoorOpen` :!label _label)
          (:`Update`
            (`SceneComponent.K2_SetRelativeLocation` _staticmeshcomponent (`KismetMathLibrary.MakeVector` (`KismetMathLibrary.Lerp` _returnvalue_x 1375.0 _sliding) 1249.0 300.0) false false)))
        (else
          (goto _label :!via `Reverse`))))))

(event `SwitchDeactive`
  ;[0 1 0.9212 0.5 40] Door gets activate once the pressure plate is stepped on (Different version of OrangeDoor opening)
  (`/Engine/EditorBlueprintResources/StandardMacros.DecrementInt` (`self.PressureSwitchActive`)
    (:`  `
      (if (>= (`self.PressureSwitchActive`) (`self.PressureSwitchNeeded`))
        (goto _label)
        (else
          (goto _label :!via `Reverse`))))))

(event `self.Box.OnComponentBeginOverlap`
  (params (OverlappedComponent :type "PrimitiveComponent Object Reference") (OtherActor :type "Actor Object Reference") (OtherComp :type "PrimitiveComponent Object Reference") (OtherBodyIndex :type Integer) (bFromSweep :type Boolean) (SweepResult :type "HitResult Structure (by ref)"))
  ;[0.15 0 0 0.5 38] Play a denied sound access when hitting the door
  (cast `/Game/ThirdPerson/Blueprints/BP_ThirdPersonCharacter` OtherActor)
  (`GameplayStatics.PlaySound2D` "/Game/Scenarios/BaseContent/Audio/S_Denied_02.S_Denied_02" 1.0 1.0 0.0 null null))

(fn `UserConstructionScript`)