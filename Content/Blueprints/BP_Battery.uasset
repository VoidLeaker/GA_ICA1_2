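; Battery actor that the player pushes in fixed-distance steps by bumping into it.
; On Hit, it rounds the player's forward vector into a push direction, and CanPush confirms with a short forward line trace that the player faces it.
; Push attaches the player to the battery with no detach shown, then the MoveBlock timeline slides it by TravelDistance from its starting location without sweeping.
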(event `self.ReceiveHit`
  (params (MyComp :type "PrimitiveComponent Object Reference") (Other :type "Actor Object Reference") (OtherComp :type "PrimitiveComponent Object Reference") (bSelfMoved :type Boolean) (HitLocation :type "Vector Structure") (HitNormal :type "Vector Structure") (NormalImpulse :type "Vector Structure") (Hit :type "HitResult Structure (by ref)"))
  ;[0.15 0 0 0.5] Pushing the object
  (if (== (`GameplayStatics.GetPlayerCharacter` 0) Other)
    (set `self.PushableDirection` (`KismetMathLibrary.MakeVector` (`KismetMathLibrary.Conv_IntToDouble` (`KismetMathLibrary.Round` (.x (`self.GetActorForwardVector` Other)))) (`KismetMathLibrary.Conv_IntToDouble` (`KismetMathLibrary.Round` (.y (`self.GetActorForwardVector` Other)))) (`KismetMathLibrary.Conv_IntToDouble` (`KismetMathLibrary.Round` (.z (`self.GetActorForwardVector` Other))))))
    (bind _canpush (`self.CanPush`))
    (if _canpush
      (`self.K2_AttachToActor` (`GameplayStatics.GetPlayerCharacter` 0) self "None" "KeepWorld" "KeepWorld" "KeepWorld" true)
      (`self.Push`))))

(event `Push`
  ;[0 1 0.1184 0.5] Adding movement to the object to allow the player to push
  (set `self.CurrentLocation` (`self.K2_GetActorLocation`))
  (bind (_direction _position) (`Timeline|MoveBlock` :!via `PlayFromStart`)
    (:`Update`
      (`self.K2_SetActorRelativeLocation` (+ (* _position (`self.PushableDirection`) (`self.TravelDistance`)) (`self.CurrentLocation`))))))

(fn `CanPush`
  (returns (CanPush :type Boolean))
  (bind _returnvalue (`GameplayStatics.GetPlayerCharacter` 0))
  (bind _returnvalue_2 (`self.K2_GetActorLocation` _returnvalue))
  ;[0 0.05979 0.15 0.5 41] Pushing the object
  (bind (_outhit _returnvalue_3) (`KismetSystemLibrary.LineTraceSingle` _returnvalue_2 (+ _returnvalue_2 (* (`self.GetActorForwardVector` _returnvalue) 100.0)) "TraceTypeQuery1" false (`|MakeArray` _returnvalue :!type "Actor Object Reference") "None" false))
  (if _returnvalue_3
    (if (== (`.HitActor` (`GameplayStatics.BreakHitResult` _outhit)) self)
      (return true)
      (else
        (return false)))
    (else
      (return false))))

(fn `UserConstructionScript`)